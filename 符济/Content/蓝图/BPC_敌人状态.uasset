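; Enemy status component that tracks health and MP, caching its BP_测试假人 (test dummy) owner on BeginPlay.
; Decrease functions subtract from each pool and return whether it is depleted; health changes also toggle 生命减少/生命增加 direction flags.
; IncreaseMP updates the player HUD's 灵墨条 bar.
; Overflowing health is set to MaxMP rather than MaxHealth, and MP's cap assigns CurrentMP to itself, leaving it unclamped.
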(event `self.ReceiveBeginPlay`
  ; 获取角色
  (bind `_asbp_测试假人` (cast `/Game/蓝图/BP_测试假人` (`self.GetOwner`)))
  (set `self.As BP 测试假人` `_asbp_测试假人`))

(fn `DecreaseHealth`
  (params (danger :type "Float (double-precision)"))
  (returns (`Is Plyaer Dead` :type Boolean))
  (if (not (<= (`self.CurrentHealth`) 0.0))
    (set `self.生命减少？` true)
    (set `self.生命增加？` false)
    (set `self.CurrentHealth` (- (`self.CurrentHealth`) danger))
    (if (<= (`self.CurrentHealth`) 0.0)
      _
      (else
        (return false))))
  (return true))

(fn `DecreaseMP`
  (params (MpUsed :type "Float (double-precision)"))
  (returns (`No MP Left` :type Boolean))
  (if (not (<= (`self.CurrentMP`) 0.0))
    (set `self.CurrentMP` (- (`self.CurrentMP`) MpUsed))
    (if (<= (`self.CurrentMP`) 0.0)
      _
      (else
        (return false))))
  (return true))

(fn `IncreaseHealth`
  (params (IncreaseHP :type "Float (double-precision)"))
  (set `self.生命减少？` false)
  (set `self.生命增加？` true)
  (set `self.CurrentHealth` (+ (`self.CurrentHealth`) IncreaseHP))
  (if (>= (`self.CurrentHealth`) (`self.MaxHealth`))
    (set `self.CurrentHealth` (`self.MaxMP`))))

(fn `IncreaseMP`
  (params (IncreaseMP :type "Float (double-precision)"))
  (bind _output_get (set `self.CurrentMP` (+ (`self.CurrentMP`) IncreaseMP)))
  (`ProgressBar.SetPercent` (`/Game/UI/WB_HUD.灵墨条` (`/Game/蓝图/玩家/BP_ThirdPersonCharacter.HUDWidget` (`self.PlayerCharacterBP`))) (/ _output_get (`self.MaxMP`)))
  (if (>= (`self.CurrentMP`) (`self.MaxMP`))
    (set `self.CurrentMP` (`self.CurrentMP`))))