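; Attack system component for BP_ThirdPersonCharacter that runs a four-hit normal melee combo on the character mesh.
; Tick polls the left mouse button while CanAttack is set, starting the combo or buffering input in SaveAttack if already attacking.
; AttackIndex selects each DoOnce-guarded, slightly delayed montage.
; 普通攻击连击, not called within this graph, continues a buffered combo or ends it, resetting the index and re-enabling Canjump.
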(event `self.ReceiveBeginPlay`
  (bind _asbp_third_person_character (cast `/Game/蓝图/BP_ThirdPersonCharacter` (`self.GetOwner`)))
  (set `self.角色网格体` (`Character.Mesh` _asbp_third_person_character)))

(event `self.ReceiveTick`
  (params (DeltaSeconds :type "Float (single-precision)"))
  ; 攻击输入
  (if (`PlayerController.IsInputKeyDown` (`GameplayStatics.GetPlayerController` 0) "LeftMouseButton")
    (if (`self.CanAttack`)
      (`self.普通攻击`))))

(event `攻击1`
  ; 攻击1
  (`/Engine/EditorBlueprintResources/StandardMacros.DoOnce` false :!label _label
    (:`Completed`
      (`KismetSystemLibrary.Delay` 0.1)
      (`|PlayMontage` (`self.角色网格体`) "/Game/Characters/林符/动画/Montages/普通攻击/Combo_Attack_02_01_Seq_Montage.Combo_Attack_02_01_Seq_Montage"
        (:`then`
          (set `self.AttackIndex` 1)
          (goto _label :!via `Reset`))))))

(event `普通攻击`
  ; 普通攻击连招
  (set `self.Canjump` false)
  (if (`self.IsAttacking`)
    (set `self.SaveAttack` true)
    (else
      (set `self.IsAttacking` true)
      (switch `int` (`self.AttackIndex`) :!label _label_2
        (:`0`
          (`self.攻击1`))
        (:`1`
          (`self.攻击2`))
        (:`2`
          (`self.攻击3`))
        (:`3`
          (`self.攻击4`))))))

(event `攻击2`
  ; 攻击2
  (`/Engine/EditorBlueprintResources/StandardMacros.DoOnce` false :!label _label_3
    (:`Completed`
      (`KismetSystemLibrary.Delay` 0.1)
      (`|PlayMontage` (`self.角色网格体`) "/Game/Characters/林符/动画/Montages/普通攻击/Combo_Attack_02_02_Seq_Montage.Combo_Attack_02_02_Seq_Montage"
        (:`then`
          (set `self.AttackIndex` 2)
          (goto _label_3 :!via `Reset`))))))

(event `普通攻击连击`
  ; 普通攻击连招
  (if (`self.SaveAttack`)
    (set `self.SaveAttack` false)
    (goto _label_2)
    (else
      (`self.终止普通攻击连击`))))

(event `攻击3`
  ; 攻击3
  (`/Engine/EditorBlueprintResources/StandardMacros.DoOnce` false :!label _label_4
    (:`Completed`
      (`KismetSystemLibrary.Delay` 0.1)
      (`|PlayMontage` (`self.角色网格体`) "/Game/Characters/林符/动画/Montages/普通攻击/Combo_Attack_02_03_Seq_Montage.Combo_Attack_02_03_Seq_Montage"
        (:`then`
          (set `self.AttackIndex` 3)
          (goto _label_4 :!via `Reset`))))))

(event `终止普通攻击连击`
  ; 停止攻击
  (set `self.IsAttacking` false)
  (set `self.AttackIndex` 0)
  (set `self.Canjump` true))

(event `攻击4`
  ; 攻击4
  (`/Engine/EditorBlueprintResources/StandardMacros.DoOnce` false :!label _label_5
    (:`Completed`
      (`KismetSystemLibrary.Delay` 0.1)
      (`|PlayMontage` (`self.角色网格体`) "/Game/Characters/林符/动画/Montages/普通攻击/Combo_Attack_02_04_Seq_Montage.Combo_Attack_02_04_Seq_Montage"
        (:`then`
          (set `self.AttackIndex` 4)
          (goto _label_5 :!via `Reset`))))))