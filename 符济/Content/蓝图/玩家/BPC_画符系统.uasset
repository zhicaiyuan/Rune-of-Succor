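; Player component for talisman-drawing (画符): right-click toggles a slow-motion drawing mode with a UI widget and mouse cursor, disabling character input.
; Entry is blocked while rolling, attacking, falling or on cooldown.
; Submitted strokes become a normalized 4x4 point-density grid, matched by Euclidean distance against same-stroke-count templates in 符库 within each one's tolerance.
; Results are only printed as skill ID or failure; recording mode prints raw features.
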(event `self.ReceiveBeginPlay`
  ; 初始化
  (bind _asbp_third_person_character (cast `/Game/蓝图/玩家/BP_ThirdPersonCharacter` (`self.GetOwner`)))
  (set `self.角色` _asbp_third_person_character)
  (set `self.玩家控制器` (`GameplayStatics.GetPlayerController` 0)))

(event `进入画符`
  (bind `_画符界面` (`self.画符界面`))
  ; 进入画符
  (bind `_画符_` (`self.守卫函数`))
  (if `_画符_`
    (set `self.是否画符中` true)
    (set `self.上次画符时间` (`KismetSystemLibrary.GetGameTimeInSeconds`))
    (`GameplayStatics.SetGlobalTimeDilation` (`self.慢动作倍率`))
    (`Actor.DisableInput` (`self.角色`) (`self.玩家控制器`))
    (bind _returnvalue (`|CreateWidget` (`self.画符界面类`) (`self.玩家控制器`)))
    (bind _output_get (set `self.画符界面` _returnvalue))
    (`UserWidget.AddToViewport` _output_get 0)
    (set `PlayerController.bShowMouseCursor` true (`self.玩家控制器`))
    (set `/Game/UI/画符界面/WBP_画符界面.画符组件` self `_画符界面`)
    (`WidgetBlueprintLibrary.SetInputMode_GameAndUIEx` (`self.玩家控制器`) `_画符界面` "DoNotLock" false)))

(event `退出画符`
  (params (`是否成功` :type Boolean))
  ; 退出画符
  (if (`self.是否画符中`)
    (set `self.是否画符中` false)
    (`GameplayStatics.SetGlobalTimeDilation` 1.0)
    (`/Engine/EditorBlueprintResources/StandardMacros.IsValid` (`self.画符界面`)
      (:`Is Valid`
        (`Widget.RemoveFromParent` (`self.画符界面`)))
      (:`Is Not Valid`
        _))
    (set `self.画符界面` null)
    (set `PlayerController.bShowMouseCursor` false (`self.玩家控制器`))
    (`Actor.EnableInput` (`self.角色`) (`self.玩家控制器`))
    (`WidgetBlueprintLibrary.SetInputMode_GameOnly` (`self.玩家控制器`))
    (if `是否成功`
      _)))

(event `提交笔画`
  (params (`笔画` :type "Array of /Game/UI/画符界面/F笔画 Structure"))
  (bind `_特征` (`self.算特征` `笔画`))
  (`KismetArrayLibrary.Array_Clear` (`self.当前特征`))
  (set `self.最佳分数` 9999.0)
  (set `self.最佳符` null)
  (if (`self.录制模式`)
    (for _array_element `_特征`
      (`KismetSystemLibrary.PrintString` (`KismetStringLibrary.Conv_DoubleToString` _array_element))
      (`self.退出画符` false))
    (else
      (set `self.当前特征` `_特征`)
      (for _array_element_2 (`self.符库`)
        (if (== (`/Game/UI/画符界面/符纸类型/DA_符.笔画数` _array_element_2) (`KismetArrayLibrary.Array_Length` `笔画`))
          (bind `_分数` (`self.比分` (`self.当前特征`) (`/Game/UI/画符界面/符纸类型/DA_符.特征` _array_element_2)))
          (if (< `_分数` (`self.最佳分数`))
            (set `self.最佳分数` `_分数`)
            (set `self.最佳符` _array_element_2))))
      (if (and (`KismetSystemLibrary.IsValid` (`self.最佳符`)) (< (`self.最佳分数`) (`/Game/UI/画符界面/符纸类型/DA_符.容差` (`self.最佳符`))))
        (`self.退出画符` false)
        (`KismetSystemLibrary.PrintString` (`KismetStringLibrary.Conv_NameToString` (`/Game/UI/画符界面/符纸类型/DA_符.技能标识` (`self.最佳符`))))
        (else
          (`self.退出画符` false)
          (`KismetSystemLibrary.PrintString` "shibai"))))))

(event `Key|RightMouseButton`
  (params (Key :type "Key Structure"))
  (:`Pressed`
    (if (`self.是否画符中`)
      (`self.退出画符` false)
      (else
        (`self.进入画符`)))))

(fn `守卫函数`
  (returns (`画符？` :type Boolean))
  (locals (`画符结果` :type Boolean))
  (if (`self.是否画符中`)
    (set `local.画符结果` false)
    (elif (`/Game/蓝图/玩家/BP_ThirdPersonCharacter.是否翻滚` (`self.角色`))
      (set `local.画符结果` false)
      (elif (`/Game/蓝图/玩家/BPC_攻击系统.IsAttacking` (`/Game/蓝图/玩家/BP_ThirdPersonCharacter.BPC_攻击系统` (`self.角色`)))
        (set `local.画符结果` false)
        (elif (`NavMovementComponent.IsFalling` (`Character.CharacterMovement` (`self.角色`)))
          (set `local.画符结果` false)
          (elif (< (- (`KismetSystemLibrary.GetGameTimeInSeconds`) (`self.上次画符时间`)) (`self.画符CD`))
            (set `local.画符结果` false)
            (else
              (set `local.画符结果` true)))))))
  (return (`local.画符结果`)))

(fn `比分`
  (params (A :type "Array of Float (double-precision)") (B :type "Array of Float (double-precision)"))
  (returns (`分数` :type "Float (double-precision)"))
  (locals (`和` :type "Float (double-precision)") (`A数组` :type "Array of Float (double-precision)") (`B数组` :type "Array of Float (double-precision)"))
  (set `local.A数组` A)
  (set `local.B数组` B)
  (if (and (== (`KismetArrayLibrary.Array_Length` A) 16) (== (`KismetArrayLibrary.Array_Length` B) 16))
    (for _index (range 16)
      (bind _returnvalue (- (`|GetArrayItem` (`local.A数组`) _index) (`|GetArrayItem` (`local.B数组`) _index)))
      (set `local.和` (+ (`local.和`) (* _returnvalue _returnvalue))))
    (return (`KismetMathLibrary.Sqrt` (`local.和`)))
    (else
      (return 9999.0))))

(fn `算特征`
  (params (`笔画` :type "Array of /Game/UI/画符界面/F笔画 Structure"))
  (returns (`特征` :type "Array of Float (double-precision)"))
  (locals (`特征结果` :type "Array of Float (double-precision)"))
  (bind `_计数` (`self.计数`))
  (for _array_element `笔画`
    (for _array_element_2 (`.点_4_63DB28E94C5AB6228670A5AA059DA87C` (break `/Game/UI/画符界面/F笔画` _array_element))
      (bind (_x _y) (`KismetMathLibrary.BreakVector2D` _array_element_2))
      (set `self.MinX` (`KismetMathLibrary.FMin` (`self.MinX`) _x))
      (set `self.MaxX` (`KismetMathLibrary.FMax` (`self.MaxX`) _x))
      (set `self.MinY` (`KismetMathLibrary.FMin` (`self.MinY`) _y))
      (set `self.MaxY` (`KismetMathLibrary.FMax` (`self.MaxY`) _y))
      (set `self.总点数` (+ (`self.总点数`) 1))))
  (if (> (`self.总点数`) 0)
    (set `self.边长` (`KismetMathLibrary.FMax` (- (`self.MaxX`) (`self.MinX`)) (- (`self.MaxY`) (`self.MinY`))))
    (if (< (`self.边长`) 1.0)
      (set `self.边长` 1.0))
    (for _ (range 16)
      (`KismetArrayLibrary.Array_Add` (`self.计数`)))
    (for _array_element_3 `笔画`
      (for _array_element_4 (`.点_4_63DB28E94C5AB6228670A5AA059DA87C` (break `/Game/UI/画符界面/F笔画` _array_element_3))
        (bind (_x_2 _y_2) (`KismetMathLibrary.BreakVector2D` _array_element_4))
        (bind _returnvalue (+ (`KismetMathLibrary.Clamp` (`KismetMathLibrary.FFloor` (* (/ (- _x_2 (`self.MinX`)) (`self.边长`)) 4.0)) 0 3) (* (`KismetMathLibrary.Clamp` (`KismetMathLibrary.FFloor` (* (/ (- _y_2 (`self.MinY`)) (`self.边长`)) 4.0)) 0 3) 4)))
        (`KismetArrayLibrary.Array_Set` `_计数` _returnvalue (+ (`|GetArrayItem` `_计数` _returnvalue) 1.0))))
    (`KismetArrayLibrary.Array_Clear` (`local.特征结果`))
    (for _index (range 16)
      (`KismetArrayLibrary.Array_Add` (`local.特征结果`) (/ (`|GetArrayItem` (`self.计数`) _index) (`KismetMathLibrary.Conv_IntToDouble` (`self.总点数`)))))
    (return (`local.特征结果`))
    (else
      (for _ (range 16)
        (`KismetArrayLibrary.Array_Add` (`local.特征结果`)))
      (return (`local.特征结果`)))))