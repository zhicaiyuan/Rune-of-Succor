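; Player status component that tracks health and MP (灵墨) for BP_ThirdPersonCharacter and writes them to its HUD bars.
; Damage and MP-spend functions return whether the pool is empty, while max-stat increases refill it and widen its bar.
; Health changes use a buffer bar: damage snaps the health bar and healing snaps the buffer, with Tick easing the other to match.
; Overhealing sets health to MaxMP, and MP gain is effectively uncapped.
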(event `self.ReceiveBeginPlay`
  (bind _asbp_third_person_character (cast `/Game/蓝图/玩家/BP_ThirdPersonCharacter` (`self.GetOwner`)))
  (set `self.PlayerCharacterBP` _asbp_third_person_character))

(event `self.ReceiveTick`
  (params (DeltaSeconds :type "Float (single-precision)"))
  (bind `_血量条` (`/Game/UI/WB_HUD.血量条` (`/Game/蓝图/玩家/BP_ThirdPersonCharacter.HUDWidget` (`self.PlayerCharacterBP`))))
  (bind `_缓冲条` (`/Game/UI/WB_HUD.缓冲条` (`/Game/蓝图/玩家/BP_ThirdPersonCharacter.HUDWidget` (`self.PlayerCharacterBP`))))
  (if (`self.生命减少？`)
    (bind _output_get (set `self.缓冲值` (`KismetMathLibrary.FInterpTo` (stale _output_get) (`ProgressBar.Percent` (`/Game/UI/WB_HUD.血量条` (`/Game/蓝图/玩家/BP_ThirdPersonCharacter.HUDWidget` (`self.PlayerCharacterBP`)))) DeltaSeconds 3.0)))
    (`ProgressBar.SetPercent` `_缓冲条` (`self.缓冲值`))
    (set `self.生命减少？` (not (`KismetMathLibrary.NearlyEqual_FloatFloat` (`ProgressBar.Percent` (`/Game/UI/WB_HUD.血量条` (`/Game/蓝图/玩家/BP_ThirdPersonCharacter.HUDWidget` (`self.PlayerCharacterBP`)))) (`ProgressBar.Percent` `_缓冲条`) 1e-05)))
    (elif (`self.生命增加？`)
      (bind _output_get_2 (set `self.缓冲值` (`KismetMathLibrary.FInterpTo` (stale _output_get_2) (`ProgressBar.Percent` (`/Game/UI/WB_HUD.缓冲条` (`/Game/蓝图/玩家/BP_ThirdPersonCharacter.HUDWidget` (`self.PlayerCharacterBP`)))) DeltaSeconds 3.0)))
      (`ProgressBar.SetPercent` `_血量条` (`self.缓冲值`))
      (set `self.生命增加？` (not (`KismetMathLibrary.NearlyEqual_FloatFloat` (`ProgressBar.Percent` (`/Game/UI/WB_HUD.缓冲条` (`/Game/蓝图/玩家/BP_ThirdPersonCharacter.HUDWidget` (`self.PlayerCharacterBP`)))) (`ProgressBar.Percent` `_血量条`) 1e-05))))))

(fn `DecreaseHealth`
  (params (danger :type "Float (double-precision)"))
  (returns (`Is Plyaer Dead` :type Boolean))
  (if (not (<= (`self.CurrentHealth`) 0.0))
    (set `self.生命减少？` true)
    (set `self.生命增加？` false)
    (bind _output_get (set `self.CurrentHealth` (- (`self.CurrentHealth`) danger)))
    (`ProgressBar.SetPercent` (`/Game/UI/WB_HUD.血量条` (`/Game/蓝图/玩家/BP_ThirdPersonCharacter.HUDWidget` (`self.PlayerCharacterBP`))) (/ _output_get (`self.MaxHealth`)))
    (if (<= (`self.CurrentHealth`) 0.0)
      _
      (else
        (return false))))
  (return true))

(fn `DecreaseMP`
  (params (MpUsed :type "Float (double-precision)"))
  (returns (`No MP Left` :type Boolean))
  (if (not (<= (`self.CurrentMP`) 0.0))
    (bind _output_get (set `self.CurrentMP` (- (`self.CurrentMP`) MpUsed)))
    (`ProgressBar.SetPercent` (`/Game/UI/WB_HUD.灵墨条` (`/Game/蓝图/玩家/BP_ThirdPersonCharacter.HUDWidget` (`self.PlayerCharacterBP`))) (/ _output_get (`self.MaxMP`)))
    (if (<= (`self.CurrentMP`) 0.0)
      _
      (else
        (return false))))
  (return true))

(fn `IncreaseHealth`
  (params (IncreaseHP :type "Float (double-precision)"))
  (set `self.生命减少？` false)
  (set `self.生命增加？` true)
  (set `self.CurrentHealth` (+ (`self.CurrentHealth`) IncreaseHP))
  (if (>= (`self.CurrentHealth`) (`self.MaxHealth`))
    (set `self.CurrentHealth` (`self.MaxMP`)))
  (`ProgressBar.SetPercent` (`/Game/UI/WB_HUD.缓冲条` (`/Game/蓝图/玩家/BP_ThirdPersonCharacter.HUDWidget` (`self.PlayerCharacterBP`))) (/ (`self.CurrentHealth`) (`self.MaxHealth`))))

(fn `IncreaseMaxHealth`
  (params (`Health Increasing` :type "Float (double-precision)"))
  (bind _output_get (set `self.MaxHealth` (+ (`self.MaxHealth`) `Health Increasing`)))
  (bind _output_get_2 (set `SizeBox.WidthOverride` (* _output_get 3.0) (`/Game/UI/WB_HUD.血量外壳` (`/Game/蓝图/玩家/BP_ThirdPersonCharacter.HUDWidget` (`self.PlayerCharacterBP`)))))
  (`ProgressBar.SetPercent` (`/Game/UI/WB_HUD.血量条` (`/Game/蓝图/玩家/BP_ThirdPersonCharacter.HUDWidget` (`self.PlayerCharacterBP`))) 1.0)
  (set `self.CurrentHealth` (`self.MaxHealth`))
  (set `SizeBox.WidthOverride` _output_get_2 (`/Game/UI/WB_HUD.血量缓冲外壳` (`/Game/蓝图/玩家/BP_ThirdPersonCharacter.HUDWidget` (`self.PlayerCharacterBP`))))
  (`ProgressBar.SetPercent` (`/Game/UI/WB_HUD.缓冲条` (`/Game/蓝图/玩家/BP_ThirdPersonCharacter.HUDWidget` (`self.PlayerCharacterBP`))) 1.0))

(fn `IncreaseMP`
  (params (IncreaseMP :type "Float (double-precision)"))
  (bind _output_get (set `self.CurrentMP` (+ (`self.CurrentMP`) IncreaseMP)))
  (`ProgressBar.SetPercent` (`/Game/UI/WB_HUD.灵墨条` (`/Game/蓝图/玩家/BP_ThirdPersonCharacter.HUDWidget` (`self.PlayerCharacterBP`))) (/ _output_get (`self.MaxMP`)))
  (if (>= (`self.CurrentMP`) (`self.MaxMP`))
    (set `self.CurrentMP` (`self.CurrentMP`))))

(fn `IncreseMaxMP`
  (params (`Increase MP` :type "Float (double-precision)"))
  (bind _output_get (set `self.MaxMP` (+ (`self.MaxMP`) `Increase MP`)))
  (bind _output_get_2 (set `self.CurrentMP` _output_get))
  (set `SizeBox.WidthOverride` (* _output_get_2 2.0) (`/Game/UI/WB_HUD.灵墨外壳` (`/Game/蓝图/玩家/BP_ThirdPersonCharacter.HUDWidget` (`self.PlayerCharacterBP`))))
  (`ProgressBar.SetPercent` (`/Game/UI/WB_HUD.灵墨条` (`/Game/蓝图/玩家/BP_ThirdPersonCharacter.HUDWidget` (`self.PlayerCharacterBP`))) 1.0)
  (set `self.CurrentMP` (`self.MaxMP`)))