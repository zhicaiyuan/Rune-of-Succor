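; Player attack component for BP_ThirdPersonCharacter that runs a left-click, four-montage sword combo and its hit detection.
; Clicks during an attack are buffered in SaveAttack, which 普通攻击连击 uses to continue or end the combo.
; A looping timer sphere-traces the blade between start/stop events, throttling hits on tagged BP_测试假人 dummies.
; Hits apply damage, four-way directional reactions, owner time-dilation hit-stop, camera shake, sound and blood.
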(event `self.ReceiveBeginPlay`
  (bind _asbp_third_person_character (cast `/Game/蓝图/玩家/BP_ThirdPersonCharacter` (`self.GetOwner`)))
  (set `self.CharacterBP` _asbp_third_person_character)
  (set `self.角色网格体` (`Character.Mesh` _asbp_third_person_character)))

(event `攻击1`
  ;[1 0.544 0.544 0.5] 连击系统
  ;; 攻击1
  (`/Engine/EditorBlueprintResources/StandardMacros.DoOnce` false :!label _label
    (:`Completed`
      (`KismetSystemLibrary.Delay` 0.1)
      (`|PlayMontage` (`self.角色网格体`) "/Game/Characters/林符/动画/Montages/普通攻击2/Combo_Attack_03_01_Seq_Montage.Combo_Attack_03_01_Seq_Montage" 1.3
        (:`then`
          (set `self.AttackIndex` 1)
          (goto _label :!via `Reset`))))))

(event `Key|LeftMouseButton`
  (params (Key :type "Key Structure"))
  ;[1 0.544 0.544 0.5] 连击系统
  ;; 攻击输入
  (:`Pressed`
    (if (`self.CanAttack`)
      (`self.普通攻击`))))

(event `普通攻击`
  ;[1 0.544 0.544 0.5] 连击系统
  ;; 普通攻击连招
  (set `self.Canjump` false)
  (if (`self.IsAttacking`)
    (set `self.SaveAttack` true)
    (else
      (set `self.IsAttacking` true)
      (switch `int` (`self.AttackIndex`) :!label _label_2
        (:`0`
          (`self.攻击1`))
        (:`1`
          (`self.攻击2`))
        (:`2`
          (`self.攻击3`))
        (:`3`
          (`self.攻击4`))))))

(event `攻击2`
  ;[1 0.544 0.544 0.5] 连击系统
  ;; 攻击2
  (`/Engine/EditorBlueprintResources/StandardMacros.DoOnce` false :!label _label_3
    (:`Completed`
      (`KismetSystemLibrary.Delay` 0.1)
      (`|PlayMontage` (`self.角色网格体`) "/Game/Characters/林符/动画/Montages/普通攻击2/Combo_Attack_03_02_Seq_Montage.Combo_Attack_03_02_Seq_Montage" 1.3
        (:`then`
          (set `self.AttackIndex` 2)
          (goto _label_3 :!via `Reset`))))))

(event `普通攻击连击`
  ;[1 0.544 0.544 0.5] 连击系统
  ;; 普通攻击连招
  (if (`self.SaveAttack`)
    (set `self.SaveAttack` false)
    (goto _label_2)
    (else
      (`self.终止普通攻击连击`))))

(event `攻击3`
  ;[1 0.544 0.544 0.5] 连击系统
  ;; 攻击3
  (`/Engine/EditorBlueprintResources/StandardMacros.DoOnce` false :!label _label_4
    (:`Completed`
      (`KismetSystemLibrary.Delay` 0.1)
      (`|PlayMontage` (`self.角色网格体`) "/Game/Characters/林符/动画/Montages/普通攻击2/Combo_Attack_03_03_Seq_Montage.Combo_Attack_03_03_Seq_Montage" 1.5
        (:`then`
          (set `self.AttackIndex` 3)
          (goto _label_4 :!via `Reset`))))))

(event `终止普通攻击连击`
  ;[1 0.544 0.544 0.5] 连击系统
  ;; 停止攻击
  (set `self.IsAttacking` false)
  (set `self.AttackIndex` 0)
  (set `self.Canjump` true))

(event `攻击4`
  ;[1 0.544 0.544 0.5] 连击系统
  ;; 攻击4
  (`/Engine/EditorBlueprintResources/StandardMacros.DoOnce` false :!label _label_5
    (:`Completed`
      (`KismetSystemLibrary.Delay` 0.1)
      (`|PlayMontage` (`self.角色网格体`) "/Game/Characters/林符/动画/Montages/普通攻击2/Combo_Attack_03_04_Seq_Montage.Combo_Attack_03_04_Seq_Montage" 1.2
        (:`then`
          (set `self.AttackIndex` 4)
          (goto _label_5 :!via `Reset`))))))

(event `开始剑追踪`
  ; 剑追踪检测n
  (bind _returnvalue (`KismetSystemLibrary.K2_SetTimerDelegate` (delegate `剑的追踪循环`) 0.01 true))
  (set `self.剑追踪循环` _returnvalue))

(event `剑的追踪循环`
  ; 剑追踪检测n
  (bind (_outhit _returnvalue) (`KismetSystemLibrary.SphereTraceSingleForObjects` (`SceneComponent.K2_GetComponentLocation` (`/Game/蓝图/玩家/BP_ThirdPersonCharacter.剑尖` (`self.CharacterBP`))) (`SceneComponent.K2_GetComponentLocation` (`/Game/蓝图/玩家/BP_ThirdPersonCharacter.剑柄` (`self.CharacterBP`))) 12.0 (`self.击中类型`)))
  (if _returnvalue
    (bind (_bblockinghit _binitialoverlap _time _distance _location _impactpoint _normal _impactnormal _physmat _hitactor) (`GameplayStatics.BreakHitResult` _outhit))
    (if (`Actor.ActorHasTag` _hitactor "可攻击的")
      (`/Engine/EditorBlueprintResources/StandardMacros.DoOnce` false :!label _label_6
        (:`Completed`
          (bind `_asbp_测试假人` (cast `/Game/蓝图/BP_测试假人` _hitactor))
          (bind (_returnvalue_roll _returnvalue_pitch _returnvalue_yaw) (`KismetMathLibrary.BreakRotator` (`KismetMathLibrary.FindLookAtRotation` (`Actor.K2_GetActorLocation` _hitactor) _impactpoint)))
          (bind (_returnvalue_roll_2 _returnvalue_pitch_2 _returnvalue_yaw_2) (`KismetMathLibrary.BreakRotator` (`Actor.K2_GetActorRotation` _hitactor)))
          (bind _returnvalue_2 (`KismetMathLibrary.NormalizeAxis` (- _returnvalue_yaw _returnvalue_yaw_2)))
          (if (and (< _returnvalue_2 45.0) (>= _returnvalue_2 -45.0))
            (set `self.受击方向` 0)
            (elif (and (>= _returnvalue_2 45.0) (< _returnvalue_2 135.0))
              (set `self.受击方向` 1)
              (elif (and (>= _returnvalue_2 -135.0) (< _returnvalue_2 -45.0))
                (set `self.受击方向` 2)
                (else
                  (set `self.受击方向` 3)))))
          (`GameplayStatics.ApplyDamage` _hitactor 10.0)
          (`/Game/蓝图/BP_测试假人.播放受击` `_asbp_测试假人` (`self.受击方向`))
          (`self.抽帧开始`)
          (`GameplayStatics.PlayWorldCameraShake` "/Game/蓝图/玩家/BP_受击摄像机震动.BP_受击摄像机震动_C" _location 0.0 2000.0)
          (`GameplayStatics.PlaySound2D` "/Game/Sword_Combat_Sounds_Pack_SFX/Sword_Hit_Human/MS_Sword_Hit_Human.MS_Sword_Hit_Human" 1.0 1.0 0.0 null null)
          (`GameplayStatics.SpawnEmitterAtLocation` "/Game/Realistic_Starter_VFX_Pack_Vol2/Particles/Blood/P_Blood_Splat_Cone.P_Blood_Splat_Cone" _location (`KismetMathLibrary.MakeRotFromXY` _normal _normal) (0.4 0.4 0.4) true "AutoRelease")
          (`KismetSystemLibrary.Delay` 0.5)
          (goto _label_6 :!via `Reset`))))))

(event `停止剑追踪`
  ; 剑追踪检测n
  (`KismetSystemLibrary.K2_ClearAndInvalidateTimerHandle` (`self.剑追踪循环`)))

(event `抽帧开始`
  ; 抽帧
  (set `Actor.CustomTimeDilation` 0.02 (`self.GetOwner`))
  (`KismetSystemLibrary.K2_SetTimerDelegate` (delegate `结束抽帧`) 0.05))

(event `结束抽帧`
  ; 抽帧
  (set `Actor.CustomTimeDilation` 1.0 (`self.GetOwner`)))