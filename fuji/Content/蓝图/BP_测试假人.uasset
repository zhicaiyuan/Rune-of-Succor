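; BP_测试假人 is a test dummy character that takes hits and stealth backstab assassinations from the player.
; AnyDamage triggers a timed hit-stop through its owner's CustomTimeDilation, knocks it up and away by the player's BPC_攻击系统 attack index, and reduces BPC敌人状态 health.
; 播放受击 plays directional hit montages for outside callers.
; 潜行背刺暗杀 plays an indexed execution montage and returns the dummy's location and rotation.
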(event `self.ReceiveAnyDamage`
  (params (Damage :type "Float (single-precision)") (DamageType :type "DamageType Object Reference") (InstigatedBy :type "Controller Object Reference") (DamageCauser :type "Actor Object Reference"))
  ; 伤害事件
  (bind _asbp_third_person_character (cast `/Game/蓝图/玩家/BP_ThirdPersonCharacter` (`GameplayStatics.GetPlayerCharacter` 0)))
  (`self.抽帧开始`)
  (bind _attackindex (`/Game/蓝图/玩家/BPC_攻击系统.AttackIndex` (`|GetArrayItem` (`self.K2_GetComponentsByClass` _asbp_third_person_character "/Game/蓝图/玩家/BPC_攻击系统.BPC_攻击系统_C"))))
  (`CombatFeelLibrary.ApplyTunedKnockback` (+ (0.0 0.0 200.0) (* (* (- (`self.K2_GetActorLocation`) (`self.K2_GetActorLocation` _asbp_third_person_character)) (1.0 1.0 0.0)) (`|GetArrayItem` (`self.击退距离`) _attackindex))) _attackindex)
  (`/Game/蓝图/BPC_敌人状态.DecreaseHealth` (`self.BPC_敌人状态`) Damage))

(event `播放受击`
  (params (`方向` :type Integer))
  ; 受击方向动画
  (`self.PlayAnimMontage` (`|GetArrayItem` (`self.受击数组`) `方向`)))

(event `抽帧开始`
  ; 抽帧
  (set `Actor.CustomTimeDilation` 0.02 (`self.GetOwner`))
  (`KismetSystemLibrary.K2_SetTimerDelegate` (delegate `结束抽帧`) 0.05))

(event `结束抽帧`
  ; 抽帧
  (set `Actor.CustomTimeDilation` 1.0 (`self.GetOwner`)))

(fn `UserConstructionScript`)

(fn `潜行背刺暗杀`
  (params (`随机动画数` :type Integer))
  (returns (`参考位置` :type "Vector Structure") (`旋转` :type "Rotator Structure"))
  (`self.PlayAnimMontage` (`|GetArrayItem` (`self.被处决数组`) `随机动画数`))
  (return (`self.K2_GetActorLocation`) (`self.K2_GetActorRotation`)))