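; Anim Notify State that marks the window in an animation during which the player character's sword trace runs.
; On begin it casts the mesh owner to BP_ThirdPersonCharacter and calls 开始剑追踪 (start sword trace) on its BPC攻击系统 attack component.
; On end it repeats the cast and calls 停止剑追踪 (stop sword trace), leaving the trace logic to that component.
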(fn `Received_NotifyBegin`
  (params (MeshComp :type "SkeletalMeshComponent Object Reference") (Animation :type "AnimSequenceBase Object Reference") (TotalDuration :type "Float (single-precision)") (EventReference :type "AnimNotifyEventReference Structure (by ref)"))
  (returns (ReturnValue :type Boolean))
  (bind _asbp_third_person_character (cast `/Game/蓝图/玩家/BP_ThirdPersonCharacter` (`ActorComponent.GetOwner` MeshComp)))
  (`/Game/蓝图/玩家/BPC_攻击系统.开始剑追踪` (`/Game/蓝图/玩家/BP_ThirdPersonCharacter.BPC_攻击系统` _asbp_third_person_character))
  (return false))

(fn `Received_NotifyEnd`
  (params (MeshComp :type "SkeletalMeshComponent Object Reference") (Animation :type "AnimSequenceBase Object Reference") (EventReference :type "AnimNotifyEventReference Structure (by ref)"))
  (returns (ReturnValue :type Boolean))
  (bind _asbp_third_person_character (cast `/Game/蓝图/玩家/BP_ThirdPersonCharacter` (`ActorComponent.GetOwner` MeshComp)))
  (`/Game/蓝图/玩家/BPC_攻击系统.停止剑追踪` (`/Game/蓝图/玩家/BP_ThirdPersonCharacter.BPC_攻击系统` _asbp_third_person_character))
  (return false))