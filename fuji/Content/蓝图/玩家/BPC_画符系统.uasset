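; Player component for talisman drawing (画符), toggled by right mouse to draw and recognize runes.
; Entry is blocked while rolling, attacking, falling or on cooldown, then slows time, disables character input and opens the drawing widget.
; Submitted strokes become features, scored against the rune library (符库) by lowest score within tolerance, filtered by stroke count and aspect ratio.
; Results are only printed; recording mode prints features instead of matching.
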(event `self.ReceiveBeginPlay`
  ; 初始化
  (bind _asbp_third_person_character (cast `/Game/蓝图/玩家/BP_ThirdPersonCharacter` (`self.GetOwner`)))
  (set `self.角色` _asbp_third_person_character)
  (set `self.玩家控制器` (`GameplayStatics.GetPlayerController` 0)))

(event `进入画符`
  (bind `_画符界面` (`self.画符界面`))
  ; 进入画符
  (bind `_画符_` (`self.守卫函数`))
  (if `_画符_`
    (set `self.是否画符中` true)
    (set `self.上次画符时间` (`KismetSystemLibrary.GetGameTimeInSeconds`))
    (`GameplayStatics.SetGlobalTimeDilation` (`self.慢动作倍率`))
    (`Actor.DisableInput` (`self.角色`) (`self.玩家控制器`))
    (bind _returnvalue (`|CreateWidget` (`self.画符界面类`) (`self.玩家控制器`)))
    (bind _output_get (set `self.画符界面` _returnvalue))
    (`UserWidget.AddToViewport` _output_get 0)
    (set `PlayerController.bShowMouseCursor` true (`self.玩家控制器`))
    (set `/Game/UI/画符界面/WBP_画符界面.画符组件` self `_画符界面`)
    (`WidgetBlueprintLibrary.SetInputMode_GameAndUIEx` (`self.玩家控制器`) `_画符界面` "DoNotLock" false)))

(event `退出画符`
  (params (`是否成功` :type Boolean))
  ; 退出画符
  (if (`self.是否画符中`)
    (set `self.是否画符中` false)
    (`GameplayStatics.SetGlobalTimeDilation` 1.0)
    (`/Engine/EditorBlueprintResources/StandardMacros.IsValid` (`self.画符界面`)
      (:`Is Valid`
        (`Widget.RemoveFromParent` (`self.画符界面`)))
      (:`Is Not Valid`
        _))
    (set `self.画符界面` null)
    (set `PlayerController.bShowMouseCursor` false (`self.玩家控制器`))
    (`Actor.EnableInput` (`self.角色`) (`self.玩家控制器`))
    (`WidgetBlueprintLibrary.SetInputMode_GameOnly` (`self.玩家控制器`))
    (if `是否成功`
      _)))

(event `提交笔画`
  (params (`笔画` :type "Array of /Game/UI/画符界面/F笔画 Structure"))
  (bind (`_特征` `_宽高比`) (`self.算特征` `笔画`))
  (`KismetArrayLibrary.Array_Clear` (`self.当前特征`))
  (set `self.最佳分数` 9999.0)
  (set `self.最佳符` null)
  (if (`self.录制模式`)
    (for _array_element `_特征`
      (`KismetSystemLibrary.PrintString` (`KismetStringLibrary.Conv_DoubleToString` _array_element))
      (`self.退出画符` false))
    (else
      (set `self.当前特征` `_特征`)
      (for _array_element_2 (`self.符库`)
        (if (== (`/Game/UI/画符界面/符纸类型/DA_符.笔画数` _array_element_2) (`KismetArrayLibrary.Array_Length` `笔画`))
          (bind `_分数` (`self.比分` (`self.当前特征`) (`/Game/UI/画符界面/符纸类型/DA_符.特征` _array_element_2)))
          (if (and (< `_分数` (`self.最佳分数`)) (< `_分数` (`/Game/UI/画符界面/符纸类型/DA_符.容差` _array_element_2)))
            (if (and (<= `_宽高比` (`/Game/UI/画符界面/符纸类型/DA_符.最大宽高比` _array_element_2)) (>= `_宽高比` (`/Game/UI/画符界面/符纸类型/DA_符.最小宽高比` _array_element_2)))
              (set `self.最佳分数` `_分数`)
              (set `self.最佳符` _array_element_2)))))
      (if (`KismetSystemLibrary.IsValid` (`self.最佳符`))
        (`self.退出画符` false)
        (`KismetSystemLibrary.PrintString` (`KismetStringLibrary.Conv_NameToString` (`/Game/UI/画符界面/符纸类型/DA_符.技能标识` (`self.最佳符`))))
        (else
          (`self.退出画符` false)
          (`KismetSystemLibrary.PrintString` "shibai"))))))

(event `Key|RightMouseButton`
  (params (Key :type "Key Structure"))
  (:`Pressed`
    (if (`self.是否画符中`)
      (`self.退出画符` false)
      (else
        (`self.进入画符`)))))

(fn `守卫函数`
  (returns (`画符？` :type Boolean))
  (locals (`画符结果` :type Boolean))
  (if (`self.是否画符中`)
    (set `local.画符结果` false)
    (elif (`/Game/蓝图/玩家/BP_ThirdPersonCharacter.是否翻滚` (`self.角色`))
      (set `local.画符结果` false)
      (elif (`/Game/蓝图/玩家/BPC_攻击系统.IsAttacking` (`/Game/蓝图/玩家/BP_ThirdPersonCharacter.BPC_攻击系统` (`self.角色`)))
        (set `local.画符结果` false)
        (elif (`NavMovementComponent.IsFalling` (`Character.CharacterMovement` (`self.角色`)))
          (set `local.画符结果` false)
          (elif (< (- (`KismetSystemLibrary.GetGameTimeInSeconds`) (`self.上次画符时间`)) (`self.画符CD`))
            (set `local.画符结果` false)
            (else
              (set `local.画符结果` true)))))))
  (return (`local.画符结果`)))

(fn `比分`
  (params (A :type "Array of Float (double-precision)") (B :type "Array of Float (double-precision)"))
  (returns (`分数` :type "Float (double-precision)"))
  (locals (`和` :type "Float (double-precision)") (`A数组` :type "Array of Float (double-precision)") (`B数组` :type "Array of Float (double-precision)"))
  (return (`RuneRecognitionLibrary.ScoreRuneFeatures` A B)))

(fn `算特征`
  (params (`笔画` :type "Array of /Game/UI/画符界面/F笔画 Structure"))
  (returns (`特征` :type "Array of Float (double-precision)") (`宽高比` :type "Float (double-precision)"))
  (locals (`特征结果` :type "Array of Float (double-precision)"))
  (bind (_features _aspectratio) (`RuneRecognitionLibrary.ExtractRuneFeatures` `笔画`))
  (return _features _aspectratio))